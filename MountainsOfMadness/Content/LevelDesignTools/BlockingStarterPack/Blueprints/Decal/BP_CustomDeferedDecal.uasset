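; A configurable decal actor from a level-design blocking pack that projects either a texture or a color, set per instance.
; The construction script builds a dynamic material instance, passes in texture, color, rotation, offset and opacity-source settings, then assigns it to the decal component.
; Texture scale is divided by the decal's world scale and size, keeping texture density independent of decal dimensions.
; It has no runtime logic.
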(event EventBeginPlay)

(event EventTick
  (params (DeltaSeconds :type Float%20%28single-precision%29)))

(fn ConstructionScript
  (bind _decal (Variables|Decal|GetDecal))
  (bind _texturescalex (Variables|Default|GetTextureScaleX))
  (bind _texturescaley (Variables|Default|GetTextureScaleY))
  (bind _returnvalue (Transformation|GetWorldScale _decal))
  (bind _decalsize (Variables|/Script/Engine.DecalComponent|GetDecalSize _decal))
  (bind _returnvalue_2 (Rendering|Material|CreateDynamicMaterialInstance (Variables|Default|GetDecalMaterial) "None" :!class /Script/Engine.KismetMaterialLibrary))
  (Variables|Default|SetDecalInstance _returnvalue_2)
  (Rendering|Material|SetScalarParameterValue (Variables|Default|GetDecalInstance) "UseTexture" (Math|Conversions|ToFloat(Boolean) (Variables|Default|GetUseTexture)) :!class /Script/Engine.MaterialInstanceDynamic)
  (Rendering|Material|SetTextureParameterValue (Variables|Default|GetDecalInstance) "Texture" (Variables|Default|GetDecalTexture))
  (Rendering|Material|SetVectorParameterValue (Variables|Default|GetDecalInstance) "Color" (Variables|Default|GetDecalColor) :!class /Script/Engine.MaterialInstanceDynamic)
  (Rendering|Material|SetScalarParameterValue (Variables|Default|GetDecalInstance) "YScale" (/ _texturescaley (* (.y _returnvalue) (.y _decalsize))) :!class /Script/Engine.MaterialInstanceDynamic)
  (Rendering|Material|SetScalarParameterValue (Variables|Default|GetDecalInstance) "XScale" (/ _texturescalex (* (.z _returnvalue) (.z _decalsize))) :!class /Script/Engine.MaterialInstanceDynamic)
  (Rendering|Material|SetScalarParameterValue (Variables|Default|GetDecalInstance) "YLocation" (* _texturescaley (/ (Variables|Default|GetTextureOffsetY) 2e+04)) :!class /Script/Engine.MaterialInstanceDynamic)
  (Rendering|Material|SetScalarParameterValue (Variables|Default|GetDecalInstance) "XLocation" (* _texturescalex (/ (Variables|Default|GetTextureOffsetX) 2e+04)) :!class /Script/Engine.MaterialInstanceDynamic)
  (Rendering|Material|SetScalarParameterValue (Variables|Default|GetDecalInstance) "ZRotation" (Variables|Default|GetTextureRotationZ) :!class /Script/Engine.MaterialInstanceDynamic)
  (Rendering|Material|SetScalarParameterValue (Variables|Default|GetDecalInstance) "TextureColorForOpacity" (Math|Conversions|ToFloat(Boolean) (Variables|Default|GetUseTextureColorForOpacity)) :!class /Script/Engine.MaterialInstanceDynamic)
  (Rendering|Components|Decal|SetDecalMaterial (Variables|Decal|GetDecal) (Variables|Default|GetDecalInstance)))