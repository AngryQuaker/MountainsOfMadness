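; BP_StackerSplineComplex is a level design construction Blueprint that places static meshes along a spline.
; When Generate is on, the construction script spaces instances by Amount or Distance, optionally treating the spline as a closed loop.
; Each transform combines seeded random jitter with the spline location, cumulative offsets, base values and optional tangent-following rotation.
; Meshes come from an array, cycled in order or picked randomly by seed.
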(event EventBeginPlay)

(event Collision|EventActorBeginOverlap
  (params (OtherActor :type Actor%20Object%20Reference)))

(event EventTick
  (params (DeltaSeconds :type Float%20%28single-precision%29)))

(fn ConstructionScript
  (bind _amount (Variables|Base|GetAmount))
  (bind _mesh (Variables|Base|GetMesh))
  (bind _seed (Variables|Base|GetSeed))
  (bind _spline (Variables|Default|GetSpline))
  (bind _mesh_2 (Variables|Base|GetMesh))
  (bind _spline_2 (Variables|Default|GetSpline))
  (bind _mode (Variables|Base|GetMode))
  (bind _distance (Variables|Base|GetDistance))
  (bind _returnvalue (Utilities|Array|Length _mesh_2))
  (bind _returnvalue_2 (== _distance 0.0))
  (bind _returnvalue_3 (Spline|GetSplineLength _spline))
  (bind _returnvalue_4 (Math|Float|SelectFloat _returnvalue_3 _distance _returnvalue_2))
  (bind _returnvalue_5 (/ _returnvalue_3 _returnvalue_4))
  (bind _returnvalue_6 (Math|Float|Floor _returnvalue_5))
  (bind _returnvalue_7 (Utilities|Select :Index _mode :NewEnumerator0 _amount :NewEnumerator1 _returnvalue_6))
  (if (Variables|Base|GetGenerate)
    (Spline|SetClosedLoop (Variables|Default|GetSpline) (Variables|Base|GetLoop) true)
    (for _index (range 0 (Math|Integer|SelectInt (- _returnvalue_7 1) _returnvalue_7 (Variables|Base|GetLoop)))
      (bind _returnvalue_8 (AddComponent|AddStaticMeshComponent false (CallFunction|CombineTransform (Math|Transform|MakeTransform (CallFunction|RandomVectorSeeded (Variables|Random|GetMinRandomLocation) (Variables|Random|GetMaxRandomLocation) _seed) (CallFunction|RandomRotSeeded (Variables|Random|GetMinRandomRotation) (Variables|Random|GetMaxRandomRotation) _seed) (CallFunction|RandomVectorSeeded (Variables|Random|GetMinRandomScale) (Variables|Random|GetMaxRandomScale) _seed)) (Math|Transform|MakeTransform (+ (Spline|GetLocationatDistanceAlongSpline _spline_2 (* _index (Utilities|Select :Index (Variables|Base|GetMode) :NewEnumerator0 (/ (Spline|GetSplineLength (Variables|Default|GetSpline)) (Math|Conversions|ToFloat(Integer) (Math|Integer|Max(Integer) (Variables|Base|GetAmount) 1))) :NewEnumerator1 (Variables|Base|GetDistance))) "Local") (+ (* (Variables|Extra|GetLocationOffset) _index) (Variables|Extra|GetLocationBase))) (Math|Rotator|SelectRotator (Math|Conversions|RotationFromXVector (Spline|GetTangentatDistanceAlongSpline _spline_2 (* _index (Utilities|Select :Index (Variables|Base|GetMode) :NewEnumerator0 (/ (Spline|GetSplineLength (Variables|Default|GetSpline)) (Math|Conversions|ToFloat(Integer) (Math|Integer|Max(Integer) (Variables|Base|GetAmount) 1))) :NewEnumerator1 (Variables|Base|GetDistance))) "Local")) (Math|Rotator|CombineRotators (* (Variables|Extra|GetRotationOffset) _index) (Variables|Extra|GetRotationBase)) (Variables|Base|GetFollowRotation)) (+ (* (Variables|Extra|GetScaleOffset) _index) (Variables|Extra|GetScaleBase))))))
      (Components|StaticMesh|SetStaticMesh _returnvalue_8 (Utilities|Select :Index (Variables|Base|GetMeshSelection) :NewEnumerator0 (Utilities|Array|Get(acopy) _mesh (Math|Integer|%(Integer) _index _returnvalue)) :NewEnumerator1 (Utilities|Array|Get(acopy) _mesh (Class|KismetMathLibrary|RandomIntegerfromStream _returnvalue (Variables|Base|GetSeed))))))))