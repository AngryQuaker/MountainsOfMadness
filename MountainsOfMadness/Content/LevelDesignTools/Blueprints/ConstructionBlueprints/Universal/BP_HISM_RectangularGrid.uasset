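; Level design construction Blueprint that fills a rectangular grid with hierarchical instanced static meshes, rebuilt in the Construction Script.
; Grid points follow the actor's forward and right vectors, optionally snapping to surfaces by line trace along a stamp direction, then shifting by a Z offset.
; Each instance gets a base rotation, randomized on all axes unless LockVerticalRotation is set, plus random uniform scale.
; Decal reception and collision response apply to the whole component.
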(event EventBeginPlay)

(event Collision|EventActorBeginOverlap
  (params (OtherActor :type Actor%20Object%20Reference)))

(event EventTick
  (params (DeltaSeconds :type Float%20%28single-precision%29)))

(fn ConstructionScript
  (bind _hierarchicalinstancedstaticmesh (Variables|Default|GetHierarchicalInstancedStaticMesh))
  (bind _singlemeshrotation (Variables|Default|GetSingleMeshRotation))
  (bind (_roll _pitch _yaw) (Math|Rotator|BreakRotator _singlemeshrotation))
  (Rendering|SetReceivesDecals _hierarchicalinstancedstaticmesh (Variables|Default|GetReceiveDecals))
  (Collision|SetCollisionResponsetoAllChannels _hierarchicalinstancedstaticmesh (Variables|Default|GetCollisionResponse))
  (for _index (range 0 (- (Variables|GridStats|GetColumns) 1))
    (LocalVariables|Setl_ColumnNumber _index)
    (for _index_2 (range 0 (- (Variables|GridStats|GetRows) 1))
      (LocalVariables|Setl_RowNumber _index_2)
      (Utilities|FlowControl|Sequence
        (:then_0
          ;[1 1 1] Get Location in Grid
          (LocalVariables|SetlclMeshLocation (+ (+ (* (Transformation|GetActorForwardVector) (* (Math|Conversions|ToFloat(Integer) (LocalVariables|Getl_ColumnNumber)) (Variables|GridStats|GetElementSize_X))) (* (Transformation|GetActorRightVector) (* (Math|Conversions|ToFloat(Integer) (LocalVariables|Getl_RowNumber)) (Variables|GridStats|GetElementSize_Y)))) (Transformation|GetWorldLocation (Variables|Default|GetDefaultSceneRoot)))))
        (:then_1
          ;[1 1 1] Stamp
          (if (Variables|Stamping|GetStampToSurface)
            (bind (_outhit _returnvalue) (Collision|LineTraceByChannel (LocalVariables|GetlclMeshLocation) (+ (LocalVariables|GetlclMeshLocation) (* (Variables|Stamping|GetScatterStampDirection) 1e+05)) "TraceTypeQuery1" false (Utilities|Array|MakeArray 0) "None" true "(R=1.000000,G=0.000000,B=0.000000,A=1.000000)" "(R=1.000000,G=0.000000,B=0.595898,A=1.000000)"))
            (if _returnvalue
              (LocalVariables|SetlclMeshLocation (.Location (Collision|BreakHitResult _outhit))))))
        (:then_2
          ;[1 1 1] Height offset
          (if (!= (Variables|GridStats|GetHeightOffset) 0.0)
            (LocalVariables|SetlclMeshLocation (Math|Vector|MakeVector (.X (Math|Vector|BreakVector (LocalVariables|GetlclMeshLocation))) (.Y (Math|Vector|BreakVector (LocalVariables|GetlclMeshLocation))) (+ (.Z (Math|Vector|BreakVector (LocalVariables|GetlclMeshLocation))) (Variables|GridStats|GetHeightOffset))))))
        (:then_3
          ;[1 1 1] Define Rot
          (if (Variables|GridStats|GetLockVerticalRotation)
            (LocalVariables|SetlclMeshRot (Math|Rotator|MakeRotator 0.0 0.0 0.0))
            (else
              (LocalVariables|SetlclMeshRot (Math|Rotator|MakeRotator (Math|Random|RandomFloatinRange 0.0 3.6e+02) (Math|Random|RandomFloatinRange 0.0 3.6e+02) (Math|Random|RandomFloatinRange 0.0 3.6e+02))))))
        (:then_4
          ;[1 1 1] Set Scale
          (LocalVariables|SetlclScale (Math|Random|RandomFloatinRange (Math|Float|Clamp(Float) (- 1.0 (Variables|GridStats|GetScaleVariance)) 0.0 1e+03) (+ (Variables|GridStats|GetScaleVariance) 1.0))))
        (:then_5
          ;[1 1 1] Spawn
          (Class|InstancedStaticMeshComponent|AddInstanceWorldSpace (Variables|Default|GetHierarchicalInstancedStaticMesh) (Math|Transform|MakeTransform (LocalVariables|GetlclMeshLocation) (Math|Rotator|MakeRotator (+ _roll (.Roll (Math|Rotator|BreakRotator (LocalVariables|GetlclMeshRot)))) (+ _pitch (.Pitch (Math|Rotator|BreakRotator (LocalVariables|GetlclMeshRot)))) (+ _yaw (.Yaw (Math|Rotator|BreakRotator (LocalVariables|GetlclMeshRot))))) (* (Math|Vector|MakeVector 1.0 1.0 1.0) (LocalVariables|GetlclScale)))))))))