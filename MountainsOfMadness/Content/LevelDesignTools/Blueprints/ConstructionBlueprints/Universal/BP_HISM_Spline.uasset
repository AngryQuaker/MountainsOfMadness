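; Level design construction Blueprint that scatters a set number of hierarchical instanced static meshes at even intervals along a spline.
; The construction script can snap each point to a surface with a line trace along a stamp direction, then adds a height offset.
; Rotation is either random, optionally yaw-only, or spline-aligned plus a fixed offset.
; Each instance gets an unseeded random uniform scale within a variance before being added in world space.
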(event EventBeginPlay)

(event Collision|EventActorBeginOverlap
  (params (OtherActor :type Actor%20Object%20Reference)))

(event EventTick
  (params (DeltaSeconds :type Float%20%28single-precision%29)))

(fn ConstructionScript
  (bind _singlemeshrotation (Variables|SplineStats|Rotation|GetSingleMeshRotation))
  (bind (_roll _pitch _yaw) (Math|Rotator|BreakRotator _singlemeshrotation))
  (for _index (range 0 (- (Variables|SplineStats|GetMeshCount) 1))
    (LocalVariables|SetlclMeshIndex _index)
    (Utilities|FlowControl|Sequence
      (:then_0
        ;[1 1 1] Get Location on Circle
        (LocalVariables|SetlclDistanceAlongSpline (* (Math|Conversions|ToFloat(Integer) (LocalVariables|GetlclMeshIndex)) (/ (Spline|GetSplineLength (Variables|Default|GetSpline)) (Math|Conversions|ToFloat(Integer) (Variables|SplineStats|GetMeshCount)))))
        (LocalVariables|SetlclMeshLocation (Spline|GetLocationatDistanceAlongSpline (Variables|Default|GetSpline) (LocalVariables|GetlclDistanceAlongSpline) "World")))
      (:then_1
        ;[1 1 1] Stamp
        (if (Variables|Stamping|GetStampToSurface)
          (bind (_outhit _returnvalue) (Collision|LineTraceByChannel (LocalVariables|GetlclMeshLocation) (+ (LocalVariables|GetlclMeshLocation) (* (Variables|Stamping|GetStampDirection) 1e+05)) "TraceTypeQuery1" false (Utilities|Array|MakeArray 0) "None" true "(R=1.000000,G=0.000000,B=0.000000,A=1.000000)" "(R=1.000000,G=0.000000,B=0.595898,A=1.000000)"))
          (if _returnvalue
            (LocalVariables|SetlclMeshLocation (.Location (Collision|BreakHitResult _outhit))))))
      (:then_2
        ;[1 1 1] Height offset
        (if (!= (Variables|SplineStats|GetHeightOffset) 0.0)
          (LocalVariables|SetlclMeshLocation (Math|Vector|MakeVector (.X (Math|Vector|BreakVector (LocalVariables|GetlclMeshLocation))) (.Y (Math|Vector|BreakVector (LocalVariables|GetlclMeshLocation))) (+ (.Z (Math|Vector|BreakVector (LocalVariables|GetlclMeshLocation))) (Variables|SplineStats|GetHeightOffset))))))
      (:then_3
        ;[1 1 1] Define Rot
        (if (Variables|SplineStats|Rotation|GetUseRandomRotation)
          (if (Variables|SplineStats|Rotation|GetLockVerticalRotation)
            (LocalVariables|SetlclMeshRot (Math|Rotator|MakeRotator 0.0 0.0 (Math|Random|RandomFloatinRange 0.0 3.6e+02)))
            (else
              (LocalVariables|SetlclMeshRot (Math|Rotator|MakeRotator (Math|Random|RandomFloatinRange 0.0 3.6e+02) (Math|Random|RandomFloatinRange 0.0 3.6e+02) (Math|Random|RandomFloatinRange 0.0 3.6e+02)))))
          (else
            (LocalVariables|SetlclMeshRot (Math|Rotator|MakeRotator (+ _roll (.Roll (Math|Rotator|BreakRotator (Spline|GetRotationatDistanceAlongSpline (Variables|Default|GetSpline) (LocalVariables|GetlclDistanceAlongSpline) "World")))) (+ _pitch (.Pitch (Math|Rotator|BreakRotator (Spline|GetRotationatDistanceAlongSpline (Variables|Default|GetSpline) (LocalVariables|GetlclDistanceAlongSpline) "World")))) (+ _yaw (.Yaw (Math|Rotator|BreakRotator (Spline|GetRotationatDistanceAlongSpline (Variables|Default|GetSpline) (LocalVariables|GetlclDistanceAlongSpline) "World")))))))))
      (:then_4
        ;[1 1 1] Set Scale
        (LocalVariables|SetlclScale (Math|Random|RandomFloatinRange (Math|Float|Clamp(Float) (- 1.0 (Variables|SplineStats|GetScaleVariance)) 0.0 1e+03) (+ (Variables|SplineStats|GetScaleVariance) 1.0))))
      (:then_5
        ;[1 1 1] Spawn
        (Class|InstancedStaticMeshComponent|AddInstanceWorldSpace (Variables|Default|GetHierarchicalInstancedStaticMesh) (Math|Transform|MakeTransform (LocalVariables|GetlclMeshLocation) (LocalVariables|GetlclMeshRot) (* (Math|Vector|MakeVector 1.0 1.0 1.0) (LocalVariables|GetlclScale))))))))