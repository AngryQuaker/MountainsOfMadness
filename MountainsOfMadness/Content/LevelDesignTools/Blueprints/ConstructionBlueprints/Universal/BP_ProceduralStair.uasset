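; Level design construction Blueprint that builds a procedural staircase from configurable step and railing meshes, materials and dimensions.
; The construction script divides length and height by step count, then adds instanced steps scaled from mesh bounds, with optional size overrides.
; Optional railing segments are instanced along both sides, pitched and stretched to the slope.
; A length-to-height ratio below the ladder threshold forces railings on; its step-scale override flag is set but never read.
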(event EventBeginPlay)

(event Collision|EventActorBeginOverlap
  (params (OtherActor :type Actor%20Object%20Reference)))

(event EventTick
  (params (DeltaSeconds :type Float%20%28single-precision%29)))

(fn ConstructionScript
  (bind _stepmesh (Variables|Steps|GetStepMesh))
  (bind _railingsmesh (Variables|Railings|GetRailingsMesh))
  (bind _railingsthickness (Variables|Railings|GetRailingsThickness))
  (bind _railings (Variables|Default|GetRailings))
  (bind _width (Variables|Geometry|GetWidth))
  (bind _returnvalue (StaticMesh|GetBounds _railingsmesh))
  (bind _returnvalue_2 (StaticMesh|GetBounds _stepmesh))
  (bind _boxextent (Math|BoxSphereBounds|BreakBoxSphereBounds _returnvalue))
  (bind _boxextent_2 (Math|BoxSphereBounds|BreakBoxSphereBounds _returnvalue_2))
  (bind _returnvalue_3 (* _boxextent 2.0))
  (bind _returnvalue_4 (* _boxextent_2 2.0))
  (bind (_x _y _z) (Math|Vector|BreakVector _returnvalue_3))
  (bind (_x_2 _y_2 _z_2) (Math|Vector|BreakVector _returnvalue_4))
  (Components|StaticMesh|SetStaticMesh (Variables|Default|GetSteps) (Variables|Steps|GetStepMesh))
  (for _index (range 0 (- (Rendering|Material|GetNumMaterials (Variables|Default|GetSteps)) 1))
    (Rendering|Material|SetMaterial (Variables|Default|GetSteps) _index (Variables|Steps|GetStepMaterial)))
  (Components|StaticMesh|SetStaticMesh (Variables|Default|GetRailings) (Variables|Railings|GetRailingsMesh))
  (for _index_2 (range 0 (- (Rendering|Material|GetNumMaterials (Variables|Default|GetRailings)) 1))
    (Rendering|Material|SetMaterial (Variables|Default|GetRailings) _index_2 (Variables|Railings|GetRailingsMaterial)))
  (if (< (/ (Variables|Geometry|GetLength) (Variables|Geometry|GetHeight)) (Variables|Default|GetLadderTreshold))
    (LocalVariables|Setl_OverrideStepScale true)
    (LocalVariables|Setl_UseRailings true)
    (else
      (LocalVariables|Setl_OverrideStepScale (Variables|Steps|Override|GetOverrideStepScale))
      (LocalVariables|Setl_UseRailings (Variables|Railings|GetUseRailings))))
  (Rendering|SetVisibility (Variables|Default|GetRailings) (LocalVariables|Getl_UseRailings) false)
  (LocalVariables|Setl_OneStepLength (/ (Variables|Geometry|GetLength) (Math|Conversions|ToFloat(Integer) (Variables|Steps|GetStepsCount))))
  (LocalVariables|Setl_OneStepHeight (/ (Variables|Geometry|GetHeight) (Math|Conversions|ToFloat(Integer) (Variables|Steps|GetStepsCount))))
  (LocalVariables|Setl_OneStepScale (Math|Vector|MakeVector (/ (Math|Float|SelectFloat (Variables|Steps|Override|GetOverrideStepLength) (LocalVariables|Getl_OneStepLength) (Variables|Steps|Override|GetOverrideStepScale)) _x_2) (/ (Variables|Geometry|GetWidth) _y_2) (/ (Math|Float|SelectFloat (Variables|Steps|Override|GetOverrideStepHeight) (LocalVariables|Getl_OneStepHeight) (Variables|Steps|Override|GetOverrideStepScale)) _z_2)))
  (LocalVariables|Setl_RailingsRotation (Math|Rotator|MakeRotator 0.0 (- (Class|KismetMathLibrary|DegAtan (/ (Variables|Geometry|GetHeight) (Variables|Geometry|GetLength))) 9e+01) 0.0))
  (LocalVariables|Setl_RailingsScale (Math|Vector|MakeVector (/ _railingsthickness _x) (/ _railingsthickness _y) (/ (Math|Float|Sqrt (+ (Math|Float|Square (LocalVariables|Getl_OneStepHeight)) (Math|Float|Square (LocalVariables|Getl_OneStepLength)))) _z)))
  (for _index_3 (range 0 (- (Variables|Steps|GetStepsCount) 1))
    (Components|InstancedStaticMesh|AddInstance (Variables|Default|GetSteps) (Math|Transform|MakeTransform (Math|Vector|MakeVector (* _index_3 (LocalVariables|Getl_OneStepLength)) 0.0 (* _index_3 (LocalVariables|Getl_OneStepHeight))) (Variables|Steps|Override|GetOverrideStepRotation) (LocalVariables|Getl_OneStepScale)))
    (if (LocalVariables|Getl_UseRailings)
      (Components|InstancedStaticMesh|AddInstance _railings (Math|Transform|MakeTransform (Math|Vector|MakeVector (* _index_3 (LocalVariables|Getl_OneStepLength)) (* _width 0.5) (+ (* _index_3 (LocalVariables|Getl_OneStepHeight)) (Variables|Railings|GetRailingsBaseShift))) (Math|Rotator|CombineRotators (LocalVariables|Getl_RailingsRotation) (Variables|Railings|GetOverrideRailingsRotation)) (LocalVariables|Getl_RailingsScale)))
      (Components|InstancedStaticMesh|AddInstance _railings (Math|Transform|MakeTransform (Math|Vector|MakeVector (* _index_3 (LocalVariables|Getl_OneStepLength)) (* _width -0.5) (+ (* _index_3 (LocalVariables|Getl_OneStepHeight)) (Variables|Railings|GetRailingsBaseShift))) (Math|Rotator|CombineRotators (LocalVariables|Getl_RailingsRotation) (Variables|Railings|GetOverrideRailingsRotation)) (LocalVariables|Getl_RailingsScale))))))