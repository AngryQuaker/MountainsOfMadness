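; BP_AngleMeasure is a level design measuring tool that displays the angle between two vectors, EndPointA and EndPointB, from the actor's origin.
; The Construction Script computes the angle in degrees from their normalized dot product and rebuilds two straight splines as the arms.
; A third spline approximates an arc between them with clamped points and tangents rotated about Z.
; A TextRender with zeroed world rotation shows the value.
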(event EventBeginPlay)

(event Collision|EventActorBeginOverlap
  (params (OtherActor :type Actor%20Object%20Reference)))

(event EventTick
  (params (DeltaSeconds :type Float%20%28single-precision%29)))

(fn ConstructionScript
  (bind _spline_arc (Variables|Default|GetSpline_arc))
  (bind _endpoint_a (Variables|Default|GetEndPoint_A))
  (bind _endpoint_b (Variables|Default|GetEndPoint_B))
  (bind _spline_a (Variables|Default|GetSpline_A))
  (bind _spline_b (Variables|Default|GetSpline_B))
  (bind _spline_a_2 (Variables|Default|GetSpline_A))
  (bind _returnvalue (* _endpoint_a _endpoint_b))
  (LocalVariables|SetAngle (Class|KismetMathLibrary|DegAcos (/ (/ (+ (.x _returnvalue) (.y _returnvalue) (.z _returnvalue)) (Math|Vector|VectorLength _endpoint_a)) (Math|Vector|VectorLength _endpoint_b))))
  (Spline|ClearSplinePoints (Variables|Default|GetSpline_A) true)
  (Spline|AddSplinePoint _spline_a (Math|Vector|MakeVector 0.0 0.0 0.0) "Local" true)
  (Spline|SetSplinePointType _spline_a 0 "Linear" true)
  (Spline|AddSplinePoint _spline_a_2 (Variables|Default|GetEndPoint_A) "Local" true)
  (Spline|SetSplinePointType _spline_a_2 1 "Linear" true)
  (Spline|AddSplinePoint _spline_b (Variables|Default|GetEndPoint_B) "Local" true)
  (Spline|SetSplinePointType _spline_b 1 "Linear" true)
  (Spline|AddSplinePoint _spline_arc (Math|Vector|ClampVectorSize (Variables|Default|GetEndPoint_A) 0.0 75.0) "Local" true)
  (Spline|SetSplinePointType _spline_arc 0 "CurveCustomTangent" true)
  (Spline|SetTangentatSplinePoint _spline_arc 0 (Math|Vector|ClampVectorSize (Math|Vector|RotateVectorAroundAxis (Variables|Default|GetEndPoint_A) 9e+01 "0, 0,1.000000") 0.0 1e+02) "Local" true)
  (Spline|AddSplinePoint _spline_arc (Math|Vector|ClampVectorSize (Variables|Default|GetEndPoint_B) 0.0 75.0) "Local" true)
  (Spline|SetSplinePointType _spline_arc 1 "CurveCustomTangent" true)
  (Spline|SetTangentatSplinePoint _spline_arc 1 (Math|Vector|ClampVectorSize (Math|Vector|RotateVectorAroundAxis (Variables|Default|GetEndPoint_B) 9e+01 "0, 0,1.000000") 0.0 1e+02) "Local" true)
  (Transformation|SetWorldRotation (Variables|Default|GetTextRender) "0, 0, 0" false false)
  (Rendering|Components|TextRender|SetText (Variables|Default|GetTextRender) (Utilities|Text|ToText(String) (Utilities|String|ToString(Float) (LocalVariables|GetAngle)))))