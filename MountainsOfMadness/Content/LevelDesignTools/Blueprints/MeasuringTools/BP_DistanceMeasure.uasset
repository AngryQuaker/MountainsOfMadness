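; BP_DistanceMeasure is a level design measuring tool that displays the distance from the actor's origin to a local EndPoint.
; The construction script rebuilds a two-point linear spline between them and places a text label at the midpoint.
; The label shows the length truncated to whole centimeters, prefixed with "~" when the true length is not a whole number.
; It has no active runtime logic.
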(event EventBeginPlay)

(event Collision|EventActorBeginOverlap
  (params (OtherActor :type Actor%20Object%20Reference)))

(event EventTick
  (params (DeltaSeconds :type Float%20%28single-precision%29)))

(fn ConstructionScript
  (bind _spline (Variables|Default|GetSpline))
  (bind _textrender (Variables|Default|GetTextRender))
  (bind _endpoint (Variables|Default|GetEndPoint))
  (bind _returnvalue (Math|Vector|VectorLength _endpoint))
  (bind _returnvalue_2 (Math|Float|Truncate _returnvalue))
  (bind _returnvalue_3 (Utilities|String|ToString(Integer) _returnvalue_2))
  (Spline|ClearSplinePoints _spline true)
  (Spline|AddSplinePoint _spline (Math|Vector|MakeVector 0.0 0.0 0.0) "Local" true)
  (Spline|SetSplinePointType _spline 0 "Linear" true)
  (Spline|AddSplinePoint _spline (Variables|Default|GetEndPoint) "Local" true)
  (Spline|SetSplinePointType _spline 1 "Linear" true)
  (Transformation|SetRelativeLocation _textrender (* (Variables|Default|GetEndPoint) 0.5) false false)
  (Rendering|Components|TextRender|SetText _textrender (Utilities|Text|ToText(String) (Utilities|String|SelectString (Utilities|String|Append "< " _returnvalue_3 "cm >") (Utilities|String|Append "< ~" _returnvalue_3 "cm >") (Math|Float|NearlyEqual(Float) _returnvalue (Math|Conversions|ToFloat(Integer) _returnvalue_2) 0.0001)))))