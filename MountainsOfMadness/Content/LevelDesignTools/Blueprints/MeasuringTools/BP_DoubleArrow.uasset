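; BP_DoubleArrow is a level design measuring-tool actor that displays a labeled arrow with two tips, the back one optionally hidden.
; Its construction script derives body length from the start-to-end distance, then lays out body, tips and description text along local X without rotating them.
; Mesh bounds convert desired thickness and tip length into scales.
; A dynamic glow material instance applies the arrow color to all three meshes.
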(event EventBeginPlay)

(event Collision|EventActorBeginOverlap
  (params (OtherActor :type Actor%20Object%20Reference)))

(event EventTick
  (params (DeltaSeconds :type Float%20%28single-precision%29)))

(fn ConstructionScript
  (bind _mainbody (Variables|Default|GetMainBody))
  (bind _description (Variables|Default|GetDescription))
  (bind _arrowtip2 (Variables|Default|GetArrowTip2))
  (bind _tiplength (Variables|Default|GetTipLength))
  (bind _arrowtip (Variables|Default|GetArrowTip))
  (bind _arrowthickness (Variables|Default|GetArrowThickness))
  (bind _staticmesh (Variables|/Script/Engine.StaticMeshComponent|GetStaticMesh _mainbody))
  (bind _staticmesh_2 (Variables|/Script/Engine.StaticMeshComponent|GetStaticMesh _arrowtip))
  (bind _returnvalue (StaticMesh|GetBounds _staticmesh))
  (bind _returnvalue_2 (StaticMesh|GetBounds _staticmesh_2))
  (bind _boxextent (Math|BoxSphereBounds|BreakBoxSphereBounds _returnvalue_2))
  (bind _boxextent_2 (Math|BoxSphereBounds|BreakBoxSphereBounds _returnvalue))
  (bind _returnvalue_3 (* _boxextent 2))
  (bind _returnvalue_4 (* _boxextent_2 2))
  (bind _returnvalue_5 (/ _arrowthickness (.x _returnvalue_4)))
  (bind _returnvalue_6 (/ _tiplength (.z _returnvalue_3)))
  (LocalVariables|Setl_TipDistance (- (Math|Vector|VectorLength (- (Variables|Default|GetEndLocation) (Variables|Default|GetStartLocation))) (* 2 (Variables|Default|GetTipLength))))
  (Transformation|SetRelativeScale3D (Variables|Default|GetMainBody) (Math|Vector|MakeVector _returnvalue_5 _returnvalue_5 (/ (LocalVariables|Getl_TipDistance) (.z _returnvalue_4))))
  (Transformation|SetRelativeLocation (Variables|Default|GetMainBody) (Math|Vector|MakeVector (Variables|Default|GetTipLength) 0.0 0.0) false false)
  (Transformation|SetRelativeLocation _description (Math|Vector|MakeVector (/ (+ (LocalVariables|Getl_TipDistance) (Variables|Default|GetTipLength)) 2.0) 0.0 0.0) false false)
  (Rendering|Components|TextRender|SetText _description (Variables|Default|GetArrowDescription))
  (Transformation|SetRelativeScale3D (Variables|Default|GetArrowTip) (Math|Vector|MakeVector _returnvalue_6 _returnvalue_6 _returnvalue_6))
  (Transformation|SetRelativeLocation (Variables|Default|GetArrowTip) (Math|Vector|MakeVector (+ (LocalVariables|Getl_TipDistance) (Variables|Default|GetTipLength)) 0.0 0.0) false false)
  (Transformation|SetRelativeLocation _arrowtip2 (Math|Vector|MakeVector (Variables|Default|GetTipLength) 0.0 0.0) false false)
  (Rendering|SetVisibility _arrowtip2 (not (Variables|Default|GetHideBackTip)) false)
  (bind _returnvalue_7 (Rendering|Material|CreateDynamicMaterialInstance "/Game/LevelDesignTools/MaterialLibrary/M_SimpleGlow_Inst.M_SimpleGlow_Inst" "None" :!class /Script/Engine.KismetMaterialLibrary))
  (Rendering|Material|SetVectorParameterValue _returnvalue_7 "Color" (Variables|Default|GetArrowColor) :!class /Script/Engine.MaterialInstanceDynamic)
  (Rendering|Material|SetMaterial (Variables|Default|GetMainBody) 0 _returnvalue_7))